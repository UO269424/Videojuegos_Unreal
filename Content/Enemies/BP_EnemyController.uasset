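; BP_EnemyController is an enemy controller that sends AI movement toward the BP_Cowboy player.
; On BeginPlay it finds and caches the cowboy, then FollowPlayer issues a single AI Move To with zero acceptance radius.
; While the cowboy is valid, Tick sets yaw-only control rotation using a look-at from cowboy to controlled pawn, so it points away from the player.
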(event `self.ReceiveBeginPlay`
  (bind _returnvalue (`GameplayStatics.GetActorOfClass` "/Game/Cowboy/BP_Cowboy.BP_Cowboy_C"))
  (set `self.Cowboy_Player` _returnvalue)
  (`self.FollowPlayer`))

(event `FollowPlayer`
  (`|AIMoveTo` null (0.0 0.0 0.0) (`self.Cowboy_Player`) 0.0))

(event `self.ReceiveTick`
  (params (DeltaSeconds :type "Float (single-precision)"))
  (bind _cowboy_player (`self.Cowboy_Player`)
    (:`then`
      (bind (_returnvalue_roll _returnvalue_pitch _returnvalue_yaw) (`KismetMathLibrary.BreakRotator` (`KismetMathLibrary.FindLookAtRotation` (`self.K2_GetActorLocation` _cowboy_player) (`self.K2_GetActorLocation` (`self.K2_GetPawn`)))))
      (`self.SetControlRotation` (`KismetMathLibrary.MakeRotator` 0.0 0.0 _returnvalue_yaw)))
    (:`else`)))

(fn `UserConstructionScript`)