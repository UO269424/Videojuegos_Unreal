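; BP_Cowboy is a player-controlled character with twin-stick style controls: independent movement, aiming and shooting.
; Move axes add movement input along fixed world X and Y, regardless of facing.
; Turn axes each update one component of LastOrientation, which sets actor rotation only when non-zero, so facing holds when aim input is released.
; The Shoot action delegates firing to BPShootingComponent.
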(event `InputAxis|MoveForward`
  (params (AxisValue :type "Float (single-precision)"))
  ;[1 1 1] Movement
  (`self.AddMovementInput` (1.0 0.0 0.0) AxisValue))

(event `InputAxis|TurnUp`
  (params (AxisValue :type "Float (single-precision)"))
  (bind (_lastorientation_x _lastorientation_y) (`KismetMathLibrary.BreakVector` (`self.LastOrientation`)))
  (bind _lastorientation (`self.LastOrientation`))
  (set `self.LastOrientation` (`KismetMathLibrary.MakeVector` AxisValue _lastorientation_y))
  (if (not (`KismetMathLibrary.Vector_IsNearlyZero` _lastorientation)) :!label _label
    (`self.K2_SetActorRotation` (`KismetMathLibrary.Conv_VectorToRotator` _lastorientation))))

(event `InputAxis|MoveRight`
  (params (AxisValue :type "Float (single-precision)"))
  ;[1 1 1] Movement
  (`self.AddMovementInput` (0.0 1.0 0.0) AxisValue))

(event `InputAxis|TurnRight`
  (params (AxisValue :type "Float (single-precision)"))
  (bind (_lastorientation_x _lastorientation_y) (`KismetMathLibrary.BreakVector` (`self.LastOrientation`)))
  (set `self.LastOrientation` (`KismetMathLibrary.MakeVector` _lastorientation_x AxisValue))
  (goto _label))

(event `InputAction|Shoot`
  (params (Key :type "Key Structure"))
  (:`Pressed`
    (`/Game/Shooting/BP_ShootingComponent.Shoot` (`self.BP_ShootingComponent`))))

(fn `UserConstructionScript`)